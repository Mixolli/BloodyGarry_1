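; BP_Sun is a light source actor that tests whether the player pawn is exposed to its PointLight, reporting only through debug prints.
; Each Tick it runs four debug-drawn Visibility traces from the light to world-space offsets below, above and either side along X of the pawn.
; Within DetectionRange, each prints minus if blocked or plus if clear.
; The Top and Bot labels are reversed relative to their Z offsets.
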(event `self.ReceiveTick`
  (params (DeltaSeconds :type "Float (single-precision)"))
  (bind _returnvalue (`GameplayStatics.GetPlayerPawn` 0))
  (bind _returnvalue_2 (`GameplayStatics.GetPlayerPawn` 0))
  (bind _returnvalue_3 (`GameplayStatics.GetPlayerPawn` 0))
  (bind _returnvalue_4 (`GameplayStatics.GetPlayerPawn` 0))
  (bind _textdur (`self.TextDur`))
  (bind _textdur_2 (`self.TextDur`))
  (bind _returnvalue_5 (`self.K2_GetActorLocation` _returnvalue_2))
  (bind _returnvalue_6 (`self.K2_GetActorLocation` _returnvalue))
  (bind _returnvalue_7 (`self.K2_GetActorLocation` _returnvalue_4))
  (bind _returnvalue_8 (`self.K2_GetActorLocation` _returnvalue_3))
  (`|ExecutionSequence`
    (:`then_0`
      (`/Engine/EditorBlueprintResources/StandardMacros.IsValid` _returnvalue_3
        (:`Is Valid`
          (set `self.PlayerInRange` (<= (`KismetMathLibrary.VSize` (- _returnvalue_8 (`self.K2_GetActorLocation`))) (`self.DetectionRange`)))
          (bind (_outhit _returnvalue_9) (`KismetSystemLibrary.LineTraceSingle` :`Start` (`SceneComponent.K2_GetComponentLocation` (`self.PointLight`)) :`End` (+ _returnvalue_8 (0.0 0.0 -75.0)) :`TraceChannel` "TraceTypeQuery1" :`DrawDebugType` "ForDuration" :`DrawTime` 0.1))
          (if (`self.PlayerInRange`)
            (if _returnvalue_9
              (`KismetSystemLibrary.PrintString` "-(Top)" true true (struct :`G` 0.66 :`B` 1.0 :`A` 1.0) _textdur)
              (else
                (`KismetSystemLibrary.PrintString` "+(Top)" true true (struct :`G` 0.66 :`B` 1.0 :`A` 1.0) _textdur)))))))
    (:`then_1`
      (`/Engine/EditorBlueprintResources/StandardMacros.IsValid` _returnvalue_2
        (:`Is Valid`
          (set `self.PlayerInRange` (<= (`KismetMathLibrary.VSize` (- _returnvalue_5 (`self.K2_GetActorLocation`))) (`self.DetectionRange`)))
          (bind (_outhit_2 _returnvalue_10) (`KismetSystemLibrary.LineTraceSingle` :`Start` (`SceneComponent.K2_GetComponentLocation` (`self.PointLight`)) :`End` (+ _returnvalue_5 (0.0 0.0 75.0)) :`TraceChannel` "TraceTypeQuery1" :`DrawDebugType` "ForDuration" :`DrawTime` 0.1))
          (if (`self.PlayerInRange`)
            (if _returnvalue_10
              (`KismetSystemLibrary.PrintString` "-(Bot)" true true (struct :`G` 0.66 :`B` 1.0 :`A` 1.0) _textdur)
              (else
                (`KismetSystemLibrary.PrintString` "+(Bot)" true true (struct :`G` 0.66 :`B` 1.0 :`A` 1.0) _textdur)))))))
    (:`then_2`
      (`/Engine/EditorBlueprintResources/StandardMacros.IsValid` _returnvalue_4
        (:`Is Valid`
          (set `self.PlayerInRange` (<= (`KismetMathLibrary.VSize` (- _returnvalue_7 (`self.K2_GetActorLocation`))) (`self.DetectionRange`)))
          (bind (_outhit_3 _returnvalue_11) (`KismetSystemLibrary.LineTraceSingle` :`Start` (`SceneComponent.K2_GetComponentLocation` (`self.PointLight`)) :`End` (+ _returnvalue_7 (50.0 0.0 0.0)) :`TraceChannel` "TraceTypeQuery1" :`DrawDebugType` "ForDuration" :`DrawTime` 0.1))
          (if (`self.PlayerInRange`)
            (if _returnvalue_11
              (`KismetSystemLibrary.PrintString` "-(SideA)" true true (struct :`G` 0.66 :`B` 1.0 :`A` 1.0) _textdur_2)
              (else
                (`KismetSystemLibrary.PrintString` "+(SideA)" true true (struct :`G` 0.66 :`B` 1.0 :`A` 1.0) _textdur_2)))))))
    (:`then_3`
      (`/Engine/EditorBlueprintResources/StandardMacros.IsValid` _returnvalue
        (:`Is Valid`
          (set `self.PlayerInRange` (<= (`KismetMathLibrary.VSize` (- _returnvalue_6 (`self.K2_GetActorLocation`))) (`self.DetectionRange`)))
          (bind (_outhit_4 _returnvalue_12) (`KismetSystemLibrary.LineTraceSingle` :`Start` (`SceneComponent.K2_GetComponentLocation` (`self.PointLight`)) :`End` (+ _returnvalue_6 (-50.0 0.0 0.0)) :`TraceChannel` "TraceTypeQuery1" :`DrawDebugType` "ForDuration" :`DrawTime` 0.1))
          (if (`self.PlayerInRange`)
            (if _returnvalue_12
              (`KismetSystemLibrary.PrintString` "-(SideB)" true true (struct :`G` 0.66 :`B` 1.0 :`A` 1.0) _textdur_2)
              (else
                (`KismetSystemLibrary.PrintString` "+(SideB)" true true (struct :`G` 0.66 :`B` 1.0 :`A` 1.0) _textdur_2)))))))))

(fn `UserConstructionScript`)